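; Player-controllable biplane pawn that routes throttle, pitch, roll and yaw axis input to its flight functions.
; Each axis has keyboard and controller bindings, with pressed flags so whichever device is active locks out the other until its value returns to zero.
; Values are forwarded tagged with their input device type.
; The construction script registers the poseable mesh, driver mesh and terrain tracker references.
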(event Input|AxisEvents|InputAxisBiplaneThrottle
  (params (AxisValue :type Float%20%28single-precision%29))
  ;[1 1 1] Input Bindings
  (if (not (Variables|Default|GetIsThrottleControllerPressed))
    (if (== AxisValue 0.0)
      (Variables|Default|SetIsThrottleKeyboardPressed false)
      (else
        (Variables|Default|SetIsThrottleKeyboardPressed true)))
    (Class|BiplanePawn|ThrottleInput AxisValue "ECT_Keyboard")))

(event Input|AxisEvents|InputAxisBiplaneThrottleController
  (params (AxisValue :type Float%20%28single-precision%29))
  ;[1 1 1] Input Bindings
  (if (not (Variables|Default|GetIsThrottleKeyboardPressed))
    (if (== AxisValue 0.0)
      (Variables|Default|SetIsThrottleControllerPressed false)
      (else
        (Variables|Default|SetIsThrottleControllerPressed true)))
    (Class|BiplanePawn|ThrottleInput AxisValue "ECT_XBox")))

(event Input|AxisEvents|InputAxisBiplanePitchDown
  (params (AxisValue :type Float%20%28single-precision%29))
  ;[1 1 1] Input Bindings
  (if (not (Variables|Default|GetIsPitchControllerPressed))
    (if (== AxisValue 0.0)
      (Variables|Default|SetIsPitchKeyboardPressed false)
      (else
        (Variables|Default|SetIsPitchKeyboardPressed true)))
    (Class|BiplanePawn|BiplanePitch AxisValue "ECT_Keyboard")))

(event Input|AxisEvents|InputAxisBiplanePitchDownController
  (params (AxisValue :type Float%20%28single-precision%29))
  ;[1 1 1] Input Bindings
  (if (not (Variables|Default|GetIsPitchKeyboardPressed))
    (if (== AxisValue 0.0)
      (Variables|Default|SetIsPitchControllerPressed false)
      (else
        (Variables|Default|SetIsPitchControllerPressed true)))
    (Class|BiplanePawn|BiplanePitch AxisValue "ECT_XBox")))

(event Input|AxisEvents|InputAxisBiplaneRollLeft
  (params (AxisValue :type Float%20%28single-precision%29))
  ;[1 1 1] Input Bindings
  (if (not (Variables|Default|GetIsRollControllerPressed))
    (if (== AxisValue 0.0)
      (Variables|Default|SetIsRollKeyboardPressed false)
      (else
        (Variables|Default|SetIsRollKeyboardPressed true)))
    (Class|BiplanePawn|BiplaneRoll AxisValue "ECT_Keyboard")))

(event Input|AxisEvents|InputAxisBiplaneRollLeftController
  (params (AxisValue :type Float%20%28single-precision%29))
  ;[1 1 1] Input Bindings
  (if (not (Variables|Default|GetIsRollKeyboardPressed))
    (if (== AxisValue 0.0)
      (Variables|Default|SetIsRollControllerPressed false)
      (else
        (Variables|Default|SetIsRollControllerPressed true)))
    (Class|BiplanePawn|BiplaneRoll AxisValue "ECT_XBox")))

(event Input|AxisEvents|InputAxisBiplaneYawLeft
  (params (AxisValue :type Float%20%28single-precision%29))
  ;[1 1 1] Input Bindings
  (if (not (Variables|Default|GetIsYawControllerPressed))
    (if (== AxisValue 0.0)
      (Variables|Default|SetIsYawKeyboardPressed false)
      (else
        (Variables|Default|SetIsYawKeyboardPressed true)))
    (Class|BiplanePawn|BiplaneYaw AxisValue "ECT_Keyboard")))

(event Input|AxisEvents|InputAxisBiplaneYawLeftController
  (params (AxisValue :type Float%20%28single-precision%29))
  ;[1 1 1] Input Bindings
  (if (not (Variables|Default|GetIsYawKeyboardPressed))
    (if (== AxisValue 0.0)
      (Variables|Default|SetIsYawControllerPressed false)
      (else
        (Variables|Default|SetIsYawControllerPressed true)))
    (Class|BiplanePawn|BiplaneYaw AxisValue "ECT_XBox")))

(fn ConstructionScript
  (Class|BiplanePawn|SetPoseableMeshReference (Variables|Default|GetPoseableMeshComponent))
  (Class|BiplanePawn|SetStaticMeshReference (Variables|Default|GetDriver))
  (Class|BiplanePawn|SetTerrainTrackerReference (Variables|Default|GetTerrainTracker)))