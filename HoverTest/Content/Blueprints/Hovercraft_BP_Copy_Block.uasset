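; Player-controlled hovercraft Blueprint that handles component setup and input for movement, hovering and camera.
; On BeginPlay it passes the static mesh to itself and four ID-numbered hover thrusters, and registers left and right rotation points.
; Input forwards movement, hover height, reset and debug-trace commands to functions defined outside these graphs.
; Camera yaw turns an azimuth gimbal and pitch turns the spring arm, with controller axes scaled by rate and delta time.
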(event EventBeginPlay
  (bind _staticmesh (Variables|Default|GetStaticMesh))
  ;[1 1 1] Index is 1-based
  (Class|Hovercraft|SetStaticMeshReference (Variables|Default|GetStaticMesh))
  (Class|HoverThruster|SetStaticMeshReference (Variables|Default|GetHoverThruster1) _staticmesh 1)
  (Class|HoverThruster|SetStaticMeshReference (Variables|Default|GetHoverThruster2) _staticmesh 2)
  (Class|HoverThruster|SetStaticMeshReference (Variables|Default|GetHoverThruster3) _staticmesh 3)
  (Class|HoverThruster|SetStaticMeshReference (Variables|Default|GetHoverThruster4) _staticmesh 4)
  (Class|Hovercraft|SetRotationPointReferences (Variables|Default|GetRight%20Rotation%20Point) (Variables|Default|GetLeft%20Rotation%20Point)))

(event Collision|EventActorBeginOverlap
  (params (OtherActor :type Actor%20Object%20Reference)))

(event EventTick
  (params (DeltaSeconds :type Float%20%28single-precision%29)))

(event Input|ActionEvents|InputActionResetHovercraft
  (params (Key :type Key%20Structure))
  ;[1 1 1] Input Actions
  (:Pressed
    (Class|Hovercraft|ResetHovercraft (Variables|Default|GetAzimuth%20Gimbal))))

(event Input|ActionEvents|InputActionToggleHoverMode
  (params (Key :type Key%20Structure))
  ;[1 1 1] Input Actions
  (:Pressed
    (Class|Hovercraft|ToggleShouldHover)))

(event Input|ActionEvents|InputActionResetHoverHeight
  (params (Key :type Key%20Structure))
  ;[1 1 1] Input Actions
  (:Pressed
    (Class|Hovercraft|ResetHoverHeight)))

(event Input|ActionEvents|InputActionIncreaseHoverHeight
  (params (Key :type Key%20Structure))
  ;[1 1 1] Input Actions
  (:Pressed
    (Class|Hovercraft|ChangeHoverHeightbySteps 1)))

(event Input|ActionEvents|InputActionDecreaseHoverHeight
  (params (Key :type Key%20Structure))
  ;[1 1 1] Input Actions
  (:Pressed
    (Class|Hovercraft|ChangeHoverHeightbySteps -1)))

(event Input|ActionEvents|InputActionDrawDebugTraces
  (params (Key :type Key%20Structure))
  ;[1 1 1] Input Actions
  (:Pressed
    (Class|Hovercraft|ToggleDrawDebugTraces)))

(event Input|AxisEvents|InputAxisMoveForward
  (params (AxisValue :type Float%20%28single-precision%29))
  ;[1 1 1] Movement
  (Class|Hovercraft|MoveForward AxisValue))

(event Input|AxisEvents|InputAxisMoveRight
  (params (AxisValue :type Float%20%28single-precision%29))
  ;[1 1 1] Movement
  (Class|Hovercraft|MoveRight AxisValue))

(event Input|AxisEvents|InputAxisRotateRight
  (params (AxisValue :type Float%20%28single-precision%29))
  ;[1 1 1] Movement
  (Class|Hovercraft|RotateRight AxisValue))

(event Input|AxisEvents|InputAxisCameraHorizontal
  (params (AxisValue :type Float%20%28single-precision%29))
  ;[1 1 1] Camera
  (Transformation|AddLocalRotation (Variables|Default|GetAzimuth%20Gimbal) (Math|Rotator|MakeRotator 0.0 0.0 AxisValue) false false))

(event Input|AxisEvents|InputAxisCameraVertical
  (params (AxisValue :type Float%20%28single-precision%29))
  ;[1 1 1] Camera
  (Transformation|AddLocalRotation (Variables|Default|GetSpringArm) (Math|Rotator|MakeRotator 0.0 AxisValue 0.0) false false))

(event Input|AxisEvents|InputAxisCameraHorizontalController
  (params (AxisValue :type Float%20%28single-precision%29))
  ;[1 1 1] Camera
  (Transformation|AddLocalRotation (Variables|Default|GetAzimuth%20Gimbal) (Math|Rotator|MakeRotator 0.0 0.0 (* AxisValue (Variables|Default|GetHorizontalCameraRateMultiplier) (Utilities|Time|GetWorldDeltaSeconds))) false false))

(event Input|AxisEvents|InputAxisCameraVerticalController
  (params (AxisValue :type Float%20%28single-precision%29))
  ;[1 1 1] Camera
  (Transformation|AddLocalRotation (Variables|Default|GetSpringArm) (Math|Rotator|MakeRotator 0.0 (* AxisValue (Variables|Default|GetVerticalCameraRateMultiplier) (Utilities|Time|GetWorldDeltaSeconds)) 0.0) false false))

(fn ConstructionScript)